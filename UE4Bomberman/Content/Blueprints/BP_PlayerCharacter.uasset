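; BP_PlayerCharacter relays second-player input to a BP_PlayerTwo actor in what appears to be a local two-player game with bombs and power-ups.
; On BeginPlay it finds that actor with GetActorOfClass and caches it as Player2.
; Its movement, bomb drop and power-up pickup input events call the matching functions on Player2, letting one Blueprint receive input for another character.
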(event `self.ReceiveBeginPlay`
  (bind _returnvalue (`GameplayStatics.GetActorOfClass` "/Game/Blueprints/BP_PlayerTwo.BP_PlayerTwo_C"))
  (set `self.Player2` _returnvalue))

(event `InputAction|DropBomb2`
  (params (Key :type "Key Structure"))
  (:`Pressed`
    (`/Game/Blueprints/BP_PlayerTwo.Drop Bomb2` (`self.Player2`))))

(event `InputAxis|MoveForward2`
  (params (AxisValue :type "Float (single-precision)"))
  (`/Game/Blueprints/BP_PlayerTwo.Move Forward2` (`self.Player2`) AxisValue))

(event `InputAxis|MoveRight2`
  (params (AxisValue :type "Float (single-precision)"))
  (`/Game/Blueprints/BP_PlayerTwo.Move Right2` (`self.Player2`) AxisValue))

(event `InputAction|Pickup PowerUp2`
  (params (Key :type "Key Structure"))
  (:`Pressed`
    (`/Game/Blueprints/BP_PlayerTwo.Pick Up Power Ups 2` (`self.Player2`))))

(fn `UserConstructionScript`)